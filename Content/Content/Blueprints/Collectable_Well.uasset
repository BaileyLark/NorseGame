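; Collectable well Blueprint that displays the player's collectable progress as a set of statues.
; The construction script gathers the statue components into the Statues array in a fixed order.
; CheckStatues reads the Collectable1 count from player info and makes entries from index zero through that count visible, printing a message for invalid ones.
; BeginPlay enables input from the first player controller, though no input events or CheckStatues calls appear here.
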(event `self.ReceiveBeginPlay`
  (`self.EnableInput` (`GameplayStatics.GetPlayerController` 0)))

(event `CheckStatues`
  (bind _player (`/Game/Content/GlobalFunctions.GetPlayerInfo`))
  (bind _output_get (set `self.Displayed` (`/Game/Content/Blueprints/PlayerCharacter.Collectable1` _player)))
  (for _index (range (+ _output_get 1))
    (bind _output (`|GetArrayItem` (`self.Statues`) _index))
    (`/Engine/EditorBlueprintResources/StandardMacros.IsValid` _output
      (:`Is Valid`
        (`SceneComponent.SetVisibility` _output true false))
      (:`Is Not Valid`
        (`KismetSystemLibrary.PrintString` "Not Valid Object")))))

(fn `UserConstructionScript`
  (`KismetArrayLibrary.Array_AddUnique` (`self.Statues`))
  (`KismetArrayLibrary.Array_AddUnique` (`self.Statues`) (`self.Statue`))
  (`KismetArrayLibrary.Array_AddUnique` (`self.Statues`) (`self.Statue1`))
  (`KismetArrayLibrary.Array_AddUnique` (`self.Statues`) (`self.Statue2`))
  (`KismetArrayLibrary.Array_AddUnique` (`self.Statues`) (`self.Statue3`))
  (`KismetArrayLibrary.Array_AddUnique` (`self.Statues`) (`self.Statue4`))
  (`KismetArrayLibrary.Array_AddUnique` (`self.Statues`) (`self.Statue5`))
  (`KismetArrayLibrary.Array_AddUnique` (`self.Statues`) (`self.Statue6`))
  (`KismetArrayLibrary.Array_AddUnique` (`self.Statues`) (`self.Statue7`))
  (`KismetArrayLibrary.Array_AddUnique` (`self.Statues`) (`self.Statue8`))
  (`KismetArrayLibrary.Array_AddUnique` (`self.Statues`) (`self.Statue10`))
  (`KismetArrayLibrary.Array_AddUnique` (`self.Statues`) (`self.Statue11`))
  (`KismetArrayLibrary.Array_AddUnique` (`self.Statues`) (`self.Statue12`)))