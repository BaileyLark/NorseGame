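; Large double door that the player buys open with coins, unlocking extra spawn locations.
; Overlapping the box deducts the Structure's cost from PlayerCharacter coins, or recolors the price text, set in the construction script, if funds are short.
; Opening plays a timeline that swings both leaves apart, hides the text and, through a DoOnce, appends the Structure's spawners to the player's PossibleLocations.
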(event `self.Box.OnComponentBeginOverlap`
  (params (OverlappedComponent :type "PrimitiveComponent Object Reference") (OtherActor :type "Actor Object Reference") (OtherComp :type "PrimitiveComponent Object Reference") (OtherBodyIndex :type Integer) (bFromSweep :type Boolean) (SweepResult :type "HitResult Structure (by ref)"))
  (bind _structure_doorcost (break `/Game/Content/Structure/DoorValues` (`self.Structure`)))
  (if (== (`GameplayStatics.GetObjectClass` OtherActor) "/Game/Content/Blueprints/PlayerCharacter.PlayerCharacter_C")
    (if (== (`self.Open`) false)
      (bind _asplayer_character (cast `/Game/Content/Blueprints/PlayerCharacter` (`GameplayStatics.GetPlayerCharacter` 0)))
      (bind _coins (`/Game/Content/Blueprints/PlayerCharacter.Coins` _asplayer_character))
      (if (>= _coins _structure_doorcost)
        (set `/Game/Content/Blueprints/PlayerCharacter.Coins` (- _coins _structure_doorcost) _asplayer_character)
        (`self.OpenDoor`)
        (set `self.Open` true)
        (else
          (`TextRenderComponent.SetTextRenderColor` (`self.TextRender`) (make `Color` 0 0 200)))))))

(event `OpenDoor`
  (bind (_structure_doorcost _structure_addspawners) (break `/Game/Content/Structure/DoorValues` (`self.Structure`)))
  (bind (_direction _newtrack_0) (`Timeline|Timeline_0` :!via `PlayFromStart`)
    (:`Update`
      (`SceneComponent.K2_SetRelativeRotation` (`self.LeftDoor`) (`KismetMathLibrary.MakeRotator` 0.0 0.0 (+ (* _newtrack_0 -90.0) -270.0)) false false)
      (`SceneComponent.K2_SetRelativeRotation` (`self.Rightdoor`) (`KismetMathLibrary.MakeRotator` 0.0 0.0 (+ (* _newtrack_0 90.0) -90.0)) false false)
      (`SceneComponent.SetVisibility` (`self.TextRender`) false false)
      (bind _asplayer_character (cast `/Game/Content/Blueprints/PlayerCharacter` (`GameplayStatics.GetPlayerCharacter` 0)))
      (`/Engine/EditorBlueprintResources/StandardMacros.DoOnce` false
        (:`Completed`
          (for _index (range (+ (`KismetArrayLibrary.Array_Length` _structure_addspawners) 1))
            (`KismetArrayLibrary.Array_Add` (`/Game/Content/Blueprints/PlayerCharacter.Possible Locations` _asplayer_character) (`|GetArrayItem` _structure_addspawners _index))))))))

(event `self.Box.OnComponentEndOverlap`
  (params (OverlappedComponent :type "PrimitiveComponent Object Reference") (OtherActor :type "Actor Object Reference") (OtherComp :type "PrimitiveComponent Object Reference") (OtherBodyIndex :type Integer))
  (`TextRenderComponent.SetTextRenderColor` (`self.TextRender`) (make `Color` 0)))

(fn `UserConstructionScript`
  (bind _structure_doorcost (break `/Game/Content/Structure/DoorValues` (`self.Structure`)))
  (`TextRenderComponent.K2_SetText` (`self.TextRender`) (`KismetTextLibrary.Conv_StringToText` (`KismetStringLibrary.Concat_StrStr` (`KismetTextLibrary.Conv_TextToString` (`KismetTextLibrary.Conv_IntToText` _structure_doorcost)) " COINS"))))