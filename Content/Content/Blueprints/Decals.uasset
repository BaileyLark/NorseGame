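; Wall decal actor that shows a configurable texture on a plane and can light up with a particle effect.
; The construction script creates a dynamic material instance from WallDecal and applies the decal texture, glow and color parameters.
; LightUp swaps in a random texture from SpawnDecals and adds a particle system, while a timeline drives the scaled Glow parameter.
; The particle component is destroyed when the timeline finishes.
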(event `LightUp`
  (`MaterialInstanceDynamic.SetTextureParameterValue` (`self.MaterialReference`) "Texture" (`KismetArrayLibrary.Array_Random` (`self.SpawnDecals`)))
  (bind _returnvalue (`AddComponent|NODE_AddParticleSystemComponent-1`))
  (bind (_direction _newtrack_0) (`Timeline|Timeline_0` :!via `PlayFromStart`)
    (:`Update`
      (`MaterialInstanceDynamic.SetScalarParameterValue` (`self.MaterialReference`) "Glow" (* _newtrack_0 3000.0)))
    (:`Finished`
      (`ActorComponent.K2_DestroyComponent` _returnvalue))))

(fn `UserConstructionScript`
  (bind _returnvalue (`KismetMaterialLibrary.CreateDynamicMaterialInstance` "/Game/Content/Mats/WallDecal.WallDecal"))
  (set `self.MaterialReference` _returnvalue)
  (`PrimitiveComponent.SetMaterial` (`self.Plane`) 0 _returnvalue)
  (`MaterialInstanceDynamic.SetTextureParameterValue` _returnvalue "Texture" (`self.Decal Texture`))
  (`MaterialInstanceDynamic.SetScalarParameterValue` _returnvalue "Glow" (`self.Glow`))
  (`MaterialInstanceDynamic.SetVectorParameterValue` _returnvalue "ColorChange" (`self.ColorChange`)))