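; Collectable is a pickup actor that adds to the player's collectable tally when its Enable event is called.
; Enable casts the player pawn to PlayerCharacter, increments Collectable1, shows the count out of a hardcoded 12 on the first top-level InfoPage widget, then destroys the actor.
; The file contains no overlap or input trigger of its own.
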(event `Enable`
  (bind _asplayer_character (cast `/Game/Content/Blueprints/PlayerCharacter` (`GameplayStatics.GetPlayerCharacter` 0)))
  (bind _output_get (set `/Game/Content/Blueprints/PlayerCharacter.Collectable1` (+ (`/Game/Content/Blueprints/PlayerCharacter.Collectable1` _asplayer_character) 1) _asplayer_character))
  (bind _foundwidgets (`WidgetBlueprintLibrary.GetAllWidgetsOfClass` "/Game/Content/UI/InfoPage.InfoPage_C"))
  (`/Game/Content/UI/InfoPage.CustomText` (`|GetArrayItem` _foundwidgets) (`KismetStringLibrary.Concat_StrStr` (`KismetStringLibrary.Conv_IntToString` _output_get) "/" "12 " "FOUND"))
  (`self.K2_DestroyActor`))

(fn `UserConstructionScript`)