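; Door is a purchasable barrier that the player opens by spending Wishes.
; The construction script shows Structure.DoorCost with a COINS label on its text render.
; When a PlayerCharacter overlaps the box, the door destroys itself and deducts the cost if the player has enough Wishes.
; Otherwise it tints the price text red, and leaving the box sets the color back to the node's default.
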(event `self.Box.OnComponentBeginOverlap`
  (params (OverlappedComponent :type "PrimitiveComponent Object Reference") (OtherActor :type "Actor Object Reference") (OtherComp :type "PrimitiveComponent Object Reference") (OtherBodyIndex :type Integer) (bFromSweep :type Boolean) (SweepResult :type "HitResult Structure (by ref)"))
  (bind _structure_doorcost (break `/Game/Content/Structure/DoorValues` (`self.Structure`)))
  (if (== (`GameplayStatics.GetObjectClass` OtherActor) "/Game/Content/Blueprints/PlayerCharacter.PlayerCharacter_C")
    (bind _asplayer_character (cast `/Game/Content/Blueprints/PlayerCharacter` (`GameplayStatics.GetPlayerCharacter` 0)))
    (bind _wishes (`/Game/Content/Blueprints/PlayerCharacter.Wishes` _asplayer_character))
    (if (>= _wishes _structure_doorcost)
      (`self.K2_DestroyActor`)
      (set `/Game/Content/Blueprints/PlayerCharacter.Wishes` (- _wishes _structure_doorcost) _asplayer_character)
      (else
        (`TextRenderComponent.SetTextRenderColor` (`self.TextRender`) (make `Color` 0 0 200))))))

(event `self.Box.OnComponentEndOverlap`
  (params (OverlappedComponent :type "PrimitiveComponent Object Reference") (OtherActor :type "Actor Object Reference") (OtherComp :type "PrimitiveComponent Object Reference") (OtherBodyIndex :type Integer))
  (`TextRenderComponent.SetTextRenderColor` (`self.TextRender`) (make `Color` 0)))

(fn `UserConstructionScript`
  (bind _structure_doorcost (break `/Game/Content/Structure/DoorValues` (`self.Structure`)))
  (`TextRenderComponent.K2_SetText` (`self.TextRender`) (`KismetTextLibrary.Conv_StringToText` (`KismetStringLibrary.Concat_StrStr` (`KismetTextLibrary.Conv_TextToString` (`KismetTextLibrary.Conv_IntToText` _structure_doorcost)) " COINS"))))