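; PrayMenu is a Blueprint that keeps a Widget component positioned near the player's look location, apparently as a pray menu.
; Every Tick it casts the player character to PlayerCharacter and teleports the widget to LookLocation plus a fixed world-space offset.
; It also sets the widget's relative roll from the negated character yaw plus a half turn, leaving BeginPlay and construction empty.
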(event `self.ReceiveBeginPlay`)

(event `self.ReceiveTick`
  (params (DeltaSeconds :type "Float (single-precision)"))
  (bind _widget (`self.Widget`))
  (bind _asplayer_character (cast `/Game/Content/Blueprints/PlayerCharacter` (`GameplayStatics.GetPlayerCharacter` 0)))
  (bind (_returnvalue_roll _returnvalue_pitch _returnvalue_yaw) (`KismetMathLibrary.BreakRotator` (`self.K2_GetActorRotation` _asplayer_character)))
  (`SceneComponent.K2_SetRelativeRotation` _widget (`KismetMathLibrary.MakeRotator` (+ (* _returnvalue_yaw -1.0) 180.0)) false false)
  (bind (_looklocation_x _looklocation_y _looklocation_z) (`KismetMathLibrary.BreakVector` (`/Game/Content/Blueprints/PlayerCharacter.LookLocation` _asplayer_character)))
  (`SceneComponent.K2_SetWorldLocation` _widget (`KismetMathLibrary.MakeVector` (+ _looklocation_x 30.0) (+ _looklocation_y 10.0) (+ _looklocation_z 5.0)) false true))

(fn `UserConstructionScript`)