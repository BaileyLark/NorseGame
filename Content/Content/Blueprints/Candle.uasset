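; Candle Blueprint with two flame planes and a point light, switched by an On flag.
; The construction script toggles their visibility and, when lit, applies the configured light temperature and intensity.
; At BeginPlay, a lit candle loops on a short Delay, randomizing the planes' Y scale around a FlameHeight offset to flicker the flame.
; A similar light-intensity flicker loop exists but is unconnected, so the light stays steady.
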(event `self.ReceiveBeginPlay`
  (if (== (`self.On`) true)
    (`SceneComponent.SetRelativeScale3D` (`self.Plane2`) (`KismetMathLibrary.MakeVector` 0.0225 (+ (`KismetMathLibrary.RandomFloatInRange` 0.07 0.1) (`self.Flame Height`)) 0.09) :!label _label)
    (`SceneComponent.SetRelativeScale3D` (`self.Plane1`) (`KismetMathLibrary.MakeVector` 0.0225 (+ (`KismetMathLibrary.RandomFloatInRange` 0.07 0.1) (`self.Flame Height`)) 0.09))
    (`KismetSystemLibrary.Delay` 0.1)
    (goto _label)))

(fn `UserConstructionScript`
  (if (== (`self.On`) true)
    (`SceneComponent.SetVisibility` (`self.Plane2`) true false)
    (`SceneComponent.SetVisibility` (`self.Plane1`) true false)
    (`SceneComponent.SetVisibility` (`self.PointLight`) true false)
    (`LightComponent.SetTemperature` (`self.PointLight`) (`self.LightHue`))
    (`LightComponent.SetIntensity` (`self.PointLight`) (`self.Light`))
    (else
      (`SceneComponent.SetVisibility` (`self.Plane2`) false false)
      (`SceneComponent.SetVisibility` (`self.Plane1`) false false)
      (`SceneComponent.SetVisibility` (`self.PointLight`) false false))))