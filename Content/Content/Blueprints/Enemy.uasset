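; Enemy actor that takes bullet damage, updates a health widget, and decrements the player's EnemiesLeft before destroying itself on death.
; On BeginPlay it randomizes walk speed with a tangent curve and, below round 30, scales health by round and lights up an overlapping Spawn-tagged decal.
; The ShowHealth volume reveals the widget while the player overlaps, with a delayed loop turning it against the player's rotation.
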(event `self.ReceiveBeginPlay`
  (bind _overlappingactors (`PrimitiveComponent.GetOverlappingActors` (`self.ShowHealth`) "/Game/Content/Blueprints/Decals.Decals_C"))
  (set `CharacterMovementComponent.MaxWalkSpeed` (* (+ 1.0 (`KismetMathLibrary.Tan` (`KismetMathLibrary.RandomFloatInRange` 0.0 1.2))) 150.0) (`self.CharacterMovement`))
  (switch `/Game/Content/EnemyType` (`self.Type`)
    (:`NewEnumerator0`
      (bind _asplayer_character (cast `/Game/Content/Blueprints/PlayerCharacter` (`GameplayStatics.GetPlayerCharacter` 0)))
      (bind _rounds (`/Game/Content/Blueprints/PlayerCharacter.Rounds` _asplayer_character))
      (if (< _rounds 30)
        (bind _output_get (set `self.FullHealth` (/ (* 0.2 (`KismetMathLibrary.Conv_IntToDouble` _rounds)) 2.0)))
        (set `self.Health` _output_get)
        (`KismetSystemLibrary.Delay` 0.3)
        (for _index (range (+ (`KismetArrayLibrary.Array_Length` _overlappingactors) 1))
          (bind _output (`|GetArrayItem` _overlappingactors _index))
          (if (`KismetSystemLibrary.IsValid` _output)
            (if (`self.ActorHasTag` _output "Spawn")
              (break))))
        (bind _asdecals (cast `/Game/Content/Blueprints/Decals` _output))
        (`/Engine/EditorBlueprintResources/StandardMacros.IsValid` _asdecals
          (:`Is Valid`
            (`/Game/Content/Blueprints/Decals.LightUp` _asdecals)))))))

(event `self.Collision.OnComponentBeginOverlap`
  (params (OverlappedComponent :type "PrimitiveComponent Object Reference") (OtherActor :type "Actor Object Reference") (OtherComp :type "PrimitiveComponent Object Reference") (OtherBodyIndex :type Integer) (bFromSweep :type Boolean) (SweepResult :type "HitResult Structure (by ref)"))
  (if (== (`GameplayStatics.GetObjectClass` OtherActor) "/Game/Content/Blueprints/Bullet.Bullet_C")
    (set `self.Health` (- (`self.Health`) 0.1))
    (bind _asenemy_health (cast `/Game/Content/UI/EnemyHealth` (`WidgetComponent.GetUserWidgetObject` (`self.Widget`))))
    (`/Game/Content/UI/EnemyHealth.Update Health` _asenemy_health (/ (`self.Health`) (`self.FullHealth`)))
    (`KismetSystemLibrary.PrintString` (`KismetStringLibrary.Concat_StrStr` "Health : " (`KismetStringLibrary.Conv_DoubleToString` (`self.Health`))))
    (`KismetSystemLibrary.PrintString` (`KismetStringLibrary.Concat_StrStr` "Full Health : " (`KismetStringLibrary.Conv_DoubleToString` (`self.Health`))))
    (cast `/Game/Content/Blueprints/PlayerCharacter` (`GameplayStatics.GetPlayerCharacter` 0))
    (if (<= (`self.Health`) 0.01)
      (bind _asplayer_character (cast `/Game/Content/Blueprints/PlayerCharacter` (`GameplayStatics.GetPlayerCharacter` 0)))
      (set `/Game/Content/Blueprints/PlayerCharacter.EnemiesLeft` (- (`/Game/Content/Blueprints/PlayerCharacter.EnemiesLeft` _asplayer_character) 1) _asplayer_character)
      (`self.K2_DestroyActor`))))

(event `self.ShowHealth.OnComponentBeginOverlap`
  (params (OverlappedComponent :type "PrimitiveComponent Object Reference") (OtherActor :type "Actor Object Reference") (OtherComp :type "PrimitiveComponent Object Reference") (OtherBodyIndex :type Integer) (bFromSweep :type Boolean) (SweepResult :type "HitResult Structure (by ref)"))
  (if (== (`GameplayStatics.GetObjectClass` OtherActor) "/Game/Content/Blueprints/PlayerCharacter.PlayerCharacter_C")
    (`SceneComponent.SetVisibility` (`self.Widget`) true false)
    (set `self.HealthToggle` true)
    (`/Engine/EditorBlueprintResources/StandardMacros.DoOnce` false :!label _label
      (:`Completed`
        (bind _asplayer_character (cast `/Game/Content/Blueprints/PlayerCharacter` (`GameplayStatics.GetPlayerCharacter` 0) :!label _label_2))
        (bind (_returnvalue_roll _returnvalue_pitch _returnvalue_yaw) (`KismetMathLibrary.BreakRotator` (`self.K2_GetActorRotation` _asplayer_character)))
        (`SceneComponent.K2_SetWorldRotation` (`self.Widget`) (`KismetMathLibrary.MakeRotator` 0.0 (* _returnvalue_pitch -1.0) (+ _returnvalue_yaw 180.0)) false false)
        (`KismetSystemLibrary.Delay` 0.05)
        (if (== (`self.HealthToggle`) true)
          (goto _label_2))))))

(event `self.ShowHealth.OnComponentEndOverlap`
  (params (OverlappedComponent :type "PrimitiveComponent Object Reference") (OtherActor :type "Actor Object Reference") (OtherComp :type "PrimitiveComponent Object Reference") (OtherBodyIndex :type Integer))
  (if (== (`GameplayStatics.GetObjectClass` OtherActor) "/Game/Content/Blueprints/PlayerCharacter.PlayerCharacter_C")
    (`SceneComponent.SetVisibility` (`self.Widget`) false false)
    (set `self.HealthToggle` false)
    (goto _label :!via `Reset`)))

(fn `UserConstructionScript`
  (`SceneComponent.SetVisibility` (`self.Widget`) false false)
  (if (`KismetMathLibrary.EqualExactly_VectorVector` (`self.K2_GetActorLocation`))
    _))