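; Coin pickup actor that adds one to the PlayerCharacter's Coins and destroys itself when that character overlaps its Box or when PickUp is called.
; When Spawn is set, it gets a random rotation at construction and a random upward, scattering force on its Cylinder at BeginPlay.
; The construction script gives the Cylinder a tinted, glowing dynamic material; a Glow timeline for animating it exists but never runs.
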(event `self.ReceiveBeginPlay`
  (if (`self.Spawn`)
    (`PrimitiveComponent.AddForce` (`self.Cylinder`) (`KismetMathLibrary.MakeVector` (`KismetMathLibrary.RandomFloatInRange` -500.0 500.0) (`KismetMathLibrary.RandomFloatInRange` -500.0 500.0) (`KismetMathLibrary.RandomFloatInRange` 500.0 1000.0)) "None" false)))

(event `Pick Up`
  (bind _asplayer_character (cast `/Game/Content/Blueprints/PlayerCharacter` (`GameplayStatics.GetPlayerCharacter` 0) :!label _label))
  (set `/Game/Content/Blueprints/PlayerCharacter.Coins` (+ (`/Game/Content/Blueprints/PlayerCharacter.Coins` _asplayer_character) 1) _asplayer_character)
  (`self.K2_DestroyActor`))

(event `self.Box.OnComponentBeginOverlap`
  (params (OverlappedComponent :type "PrimitiveComponent Object Reference") (OtherActor :type "Actor Object Reference") (OtherComp :type "PrimitiveComponent Object Reference") (OtherBodyIndex :type Integer) (bFromSweep :type Boolean) (SweepResult :type "HitResult Structure (by ref)"))
  (if (== (`GameplayStatics.GetObjectClass` OtherActor) "/Game/Content/Blueprints/PlayerCharacter.PlayerCharacter_C")
    (goto _label)))

(fn `UserConstructionScript`
  (locals (NewLocalVar_0 :type "MaterialInstanceDynamic Object Reference"))
  (if (`self.Spawn`)
    (`self.K2_SetActorRotation` (`KismetMathLibrary.RandomRotator` true))
    (else
      (`self.K2_SetActorRotation` (struct))))
  (bind _returnvalue (`KismetMaterialLibrary.CreateDynamicMaterialInstance` "/Game/Content/Mats/Glow.Glow"))
  (set `self.MatRef` _returnvalue)
  (`MaterialInstanceDynamic.SetVectorParameterValue` _returnvalue "Color" (struct :`R` 0.890625 :`G` 0.883325 :`B` 0.691162 :`A` 1.0))
  (`MaterialInstanceDynamic.SetScalarParameterValue` _returnvalue "Glow" 2.0)
  (`PrimitiveComponent.SetMaterial` (`self.Cylinder`) 0 _returnvalue))