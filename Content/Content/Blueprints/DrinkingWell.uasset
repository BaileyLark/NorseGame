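; A drinking well the player uses with F to restore up to 25 health per drink from a limited water supply.
; An overlap volume tracks the player and shows a DrinkWater widget of remaining drinks; drinking also requires the well to be enabled.
; UpdateItem ties water height, light intensity and water and steam visibility to WaterLeft, while external events refill or toggle the well.
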(event `AddWater`
  (set `self.WaterLeft` 3)
  (`self.UpdateItem`))

(event `Enable Well`
  (params (Toggle :type Boolean))
  (set `self.Enabled?` Toggle))

(event `self.ReceiveBeginPlay`
  (`|ExecutionSequence`
    (:`then_0`
      (set `self.WaterLeft` 2)
      (`SceneComponent.K2_SetRelativeLocation` (`self.Water2`) (`KismetMathLibrary.MakeVector` -14.0 0.0 (`KismetMathLibrary.Conv_IntToDouble` (+ (`self.WaterLeft`) 27))) false false))
    (:`then_1`
      (`KismetSystemLibrary.Delay` 5.0))))

(event `Key|F` :consume false
  (params (Key :type "Key Structure"))
  (:`Pressed`
    (if (and (and (`self.Enabled?`) (`self.Proxmity`)) (> (`self.WaterLeft`) -1))
      (bind _asplayer_character (cast `/Game/Content/Blueprints/PlayerCharacter` (`GameplayStatics.GetPlayerCharacter` 0)))
      (bind _health (`/Game/Content/Blueprints/PlayerCharacter.Health` _asplayer_character))
      (if (< _health 100.0)
        (for _ (range 1 26)
          (if (>= _health 100.0)
            (break)
            (else
              (set `/Game/Content/Blueprints/PlayerCharacter.Health` (+ _health 1.0) _asplayer_character))))
        (`/Game/Content/UI/DrinkWater.Update ` (stale `self.Proximity.OnComponentBeginOverlap` _returnvalue) (`self.WaterLeft`))
        (`SceneComponent.K2_SetRelativeLocation` (`self.Water2`) (`KismetMathLibrary.MakeVector` -14.0 0.0 (`KismetMathLibrary.Conv_IntToDouble` (+ (`self.WaterLeft`) 27))) false false)
        (set `self.WaterLeft` (- (`self.WaterLeft`) 1))
        (`self.UpdateItem`)))))

(event `UpdateItem`
  (bind _steam (`self.Steam`))
  (if (>= (`self.WaterLeft`) 0)
    (`SceneComponent.SetVisibility` _steam true false)
    (`SceneComponent.SetVisibility` (`self.Water2`) true false)
    (`LightComponent.SetIntensity` (`self.PointLight`) (`KismetMathLibrary.Conv_IntToDouble` (* (`self.WaterLeft`) 750)))
    (`SceneComponent.K2_SetRelativeLocation` (`self.Water2`) (`KismetMathLibrary.MakeVector` -14.0 0.0 (`KismetMathLibrary.Conv_IntToDouble` (+ (`self.WaterLeft`) 27))) false false)
    (else
      (`SceneComponent.SetVisibility` _steam false false)
      (`SceneComponent.SetVisibility` (`self.Water2`) false false)
      (`/Engine/EditorBlueprintResources/StandardMacros.DoOnce` false))))

(event `self.Proximity.OnComponentBeginOverlap`
  (params (OverlappedComponent :type "PrimitiveComponent Object Reference") (OtherActor :type "Actor Object Reference") (OtherComp :type "PrimitiveComponent Object Reference") (OtherBodyIndex :type Integer) (bFromSweep :type Boolean) (SweepResult :type "HitResult Structure (by ref)"))
  (if (== (`GameplayStatics.GetObjectClass` OtherActor) "/Game/Content/Blueprints/PlayerCharacter.PlayerCharacter_C")
    (set `self.Proxmity` true)
    (bind _returnvalue (`|CreateWidget` "/Game/Content/UI/DrinkWater.DrinkWater_C"))
    (`UserWidget.AddToViewport` _returnvalue 0)
    (`/Game/Content/UI/DrinkWater.Update ` _returnvalue (`self.WaterLeft`))))

(event `self.Proximity.OnComponentEndOverlap`
  (params (OverlappedComponent :type "PrimitiveComponent Object Reference") (OtherActor :type "Actor Object Reference") (OtherComp :type "PrimitiveComponent Object Reference") (OtherBodyIndex :type Integer))
  (if (== (`GameplayStatics.GetObjectClass` OtherActor) "/Game/Content/Blueprints/PlayerCharacter.PlayerCharacter_C")
    (set `self.Proxmity` false)
    (`Widget.RemoveFromParent` (stale `self.Proximity.OnComponentBeginOverlap` _returnvalue))
    (`KismetSystemLibrary.PrintString` "dISABLED!")))

(fn `UserConstructionScript`)